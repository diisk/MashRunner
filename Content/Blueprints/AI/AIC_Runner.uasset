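; AIC_Runner is an AI controller that drives a BP_Runner pawn by faking player power inputs.
; On possession it stores the runner, and from BeginPlay it schedules input on a one-shot timer with a random delay between minimum and maximum values.
; SimulateInput uses a FlipFlop to alternate left and right power calls on the runner, rescheduling the timer after each one.
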(event Custom|SimulateInput
  (bind _owningrunner (Variables|Default|GetOwningRunner))
  (Utilities|FlowControl|FlipFlop
    (:A
      (Default|SimulatePowerLeft _owningrunner))
    (:B
      (Default|SimulatePowerRight _owningrunner)))
  (CallFunction|SimulateInputwithDelay))

(event EventBeginPlay
  (CallFunction|SimulateInputwithDelay))

(event EventPossess
  (params (PossessedPawn :type Pawn%20Object%20Reference))
  (bind _asbp_runner (Utilities|Casting|CastToBP_Runner PossessedPawn))
  (Variables|Default|SetOwningRunner _asbp_runner))

(fn ConstructionScript)

(fn SimulateInputwithDelay
  (Utilities|Time|SetTimerbyEvent (EventDispatchers|CreateEvent :!event Custom|SimulateInput) (Math|Random|RandomFloatinRange (Variables|Default|GetMinInputDelay) (Variables|Default|GetMaxInputDelay))))